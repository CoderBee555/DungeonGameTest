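; Interactable hinged door that the player can open and close, with an on-screen key prompt.
; A trigger box registers the door as Player_1's InteractableObject and shows the prompt, clearing both when the player leaves.
; Interact toggles IsOpen, plays or reverses a timeline that drives the DoorPivot yaw, and recreates the Message widget with the matching open or close text.
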(event OnComponentBeginOverlap(Box)
  (params (OverlappedComponent :type Primitive%20Component%20Object%20Reference) (OtherActor :type Actor%20Object%20Reference) (OtherComp :type Primitive%20Component%20Object%20Reference) (OtherBodyIndex :type Integer) (bFromSweep :type Boolean) (SweepResult :type Hit%20Result%20Structure%20%28by%20ref%29))
  ;[1 1 1] Trigger
  (bind _asplayer_1 (Utilities|Casting|CastToPlayer_1 OtherActor))
  (Variables|/Game/ThirdPersonBP/Blueprints/Player_1.Player_1_C|SetInteractableObject _asplayer_1 self)
  (CallFunction|ShowMessage))

(event OnComponentEndOverlap(Box)
  (params (OverlappedComponent :type Primitive%20Component%20Object%20Reference) (OtherActor :type Actor%20Object%20Reference) (OtherComp :type Primitive%20Component%20Object%20Reference) (OtherBodyIndex :type Integer))
  ;[1 1 1] Trigger
  (bind _asplayer_1 (Utilities|Casting|CastToPlayer_1 OtherActor))
  (Variables|/Game/ThirdPersonBP/Blueprints/Player_1.Player_1_C|SetInteractableObject _asplayer_1 0)
  (Widget|RemovefromParent (Variables|Default|GetWidget)))

(event Custom|Open
  ;[1 1 1] Open / Close Animation
  (bind _rotation (Timeline|Open%20Close%20Sequence Play)
    (:Update
      (Transformation|SetRelativeRotation (Variables|Default|GetDoor_Pivot) (Math|Rotator|MakeRotator 0.0 0.0 _rotation) false false))))

(event Custom|Close
  ;[1 1 1] Open / Close Animation
  (bind _rotation (Timeline|Open%20Close%20Sequence Reverse)
    (:Update
      (Transformation|SetRelativeRotation (Variables|Default|GetDoor_Pivot) (Math|Rotator|MakeRotator 0.0 0.0 _rotation) false false))))

(event EventBeginPlay)

(event EventInteract
  ;[1 1 1] On Interact
  (if (Variables|Default|GetisOpen)
    (Variables|Default|SetisOpen false)
    (CallFunction|Close)
    (else
      (Variables|Default|SetisOpen true)
      (CallFunction|Open)))
  (Widget|RemovefromParent (Variables|Default|GetWidget))
  (CallFunction|ShowMessage))

(fn ConstructionScript)

(fn ShowMessage
  (if (Variables|Default|GetisOpen)
    (bind _returnvalue (UserInterface|CreateWidget "/Game/Blueprints/UI_Blueprints/Message.Message_C" 0 "Press [E] to close the door"))
    (bind _output_get (Variables|Default|SetWidget _returnvalue))
    (UserInterface|Viewport|AddtoViewport _output_get 0)
    (else
      (bind _returnvalue_2 (UserInterface|CreateWidget "/Game/Blueprints/UI_Blueprints/Message.Message_C" 0 "Press [E] to open the door"))
      (bind _output_get_2 (Variables|Default|SetWidget _returnvalue_2))
      (UserInterface|Viewport|AddtoViewport _output_get_2 0))))