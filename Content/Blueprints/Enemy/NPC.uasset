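; Enemy NPC Blueprint with a health bar widget and a simple rotation-based attack.
; Tick pushes max and current health into the Health widget every frame and destroys the actor when current health reaches zero.
; The Attack event alternates through a FlipFlop between playing and reversing a timeline that drives the yaw of an arrow component.
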(event Custom|Attack
  (bind _arrow1 (Variables|Default|GetArrow1))
  (bind _relativerotation (Variables|/Script/Engine.SceneComponent|GetRelativeRotation _arrow1))
  (bind (_roll _pitch) (Math|Rotator|BreakRotator _relativerotation))
  ;[1 1 1] Attack
  (Utilities|FlowControl|FlipFlop
    (:A
      (bind _rotation (Timeline|Timeline_0 Play)
        (:Update
          (Transformation|SetRelativeRotation _arrow1 (Math|Rotator|MakeRotator _roll _pitch _rotation) false false))))
    (:B
      (Timeline|Timeline_0 Reverse))))

(event EventTick
  (params (DeltaSeconds :type Float%20%28single-precision%29))
  (bind _ashealth (Utilities|Casting|CastToHealth (UserInterface|GetWidget (Variables|Default|GetHealthBar))))
  (Variables|/Game/Blueprints/UI_Blueprints/Health.Health_C|SetMax%20Health _ashealth (Variables|Default|GetMaxHealth))
  (Variables|/Game/Blueprints/UI_Blueprints/Health.Health_C|SetCurrent%20Health _ashealth (Variables|Default|GetCurrentHealth))
  (if (<= (Variables|Default|GetCurrentHealth) 0.0)
    (Actor|DestroyActor)))

(fn ConstructionScript)