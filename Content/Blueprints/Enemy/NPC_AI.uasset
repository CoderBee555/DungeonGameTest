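; AI controller for patrolling NPC enemies that detect the player.
; On BeginPlay it runs the NPC_BT behavior tree and seeds the blackboard with the pawn's patrol path looping flag and wait time, plus a starting direction.
; AI Perception updates set CanSeePlayer whenever the Player_1 target is sensed or lost, leaving the resulting behavior to the tree.
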(event OnTargetPerceptionUpdated(AIPerception)
  (params (Actor :type Actor%20Object%20Reference) (Stimulus :type AI%20Stimulus%20Structure))
  (Utilities|Casting|CastToPlayer_1 Actor)
  (AI|Components|Blackboard|SetValueasBool (AI|GetBlackboard 0) (Utilities|Name|MakeLiteralName "CanSeePlayer") (.bSuccessfullySensed (Utilities|Struct|BreakAIStimulus Stimulus))))

(event EventBeginPlay
  (AI|RunBehaviorTree "/Game/Blueprints/Enemy/NPC_BT.NPC_BT")
  (bind _asnpc (Utilities|Casting|CastToNPC (Pawn|GetControlledPawn)))
  (Variables|Default|SetMy%20Pawn _asnpc)
  (AI|Components|Blackboard|SetValueasBool (AI|GetBlackboard 0) (Utilities|Name|MakeLiteralName "PathLooping") (Variables|/Game/Blueprints/Enemy/PatrolPath.PatrolPath_C|GetIsLooping (Variables|/Game/Blueprints/Enemy/NPC.NPC_C|GetPatrolPath (Variables|Default|GetMy%20Pawn))))
  (Class|BlackboardComponent|SetValueasInt (AI|GetBlackboard 0) (Utilities|Name|MakeLiteralName "Direction") 1)
  (AI|Components|Blackboard|SetValueasFloat (AI|GetBlackboard 0) (Utilities|Name|MakeLiteralName "WaitTime") (Variables|/Game/Blueprints/Enemy/PatrolPath.PatrolPath_C|GetWaitTime (Variables|/Game/Blueprints/Enemy/NPC.NPC_C|GetPatrolPath (Variables|Default|GetMy%20Pawn)))))

(event EventTick
  (params (DeltaSeconds :type Float%20%28single-precision%29)))

(fn ConstructionScript)