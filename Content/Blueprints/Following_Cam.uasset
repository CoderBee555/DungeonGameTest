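; Following camera actor that tracks Player1 from a fixed elevated offset while single-player mode is on.
; Each Tick it teleports to the player's location plus that offset, keeping its own rotation, with no smoothing.
; It also prints mouse X and Y axis values as debug text, without using them to move the camera.
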(event EventBeginPlay)

(event Collision|EventActorBeginOverlap
  (params (OtherActor :type Actor%20Object%20Reference)))

(event EventTick
  (params (DeltaSeconds :type Float%20%28single-precision%29))
  (bind _self self)
  (if (Variables|Default|GetIsSinglePlayerMode?)
    (Transformation|Teleport _self (+ (Transformation|GetActorLocation (Variables|Default|GetPlayer_1)) "-500.000000,-500.000000,600.000000") (Transformation|GetActorRotation _self))
    (Development|PrintString (Utilities|String|Append "Mosue x: " (Utilities|String|ToString(Float) (Class|Actor|GetInputAxisKeyValue))))
    (Development|PrintString (Utilities|String|Append "Mosue y: " (Utilities|String|ToString(Float) (Class|Actor|GetInputAxisKeyValue))))))

(fn ConstructionScript)